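; Lap checkpoint actor that marks a point pawns pass through during a lap.
; On BeginPlay it increments LapPointNumber on the Mk game mode, so the mode holds a count of placed checkpoints.
; When a pawn overlaps its Box, it passes itself to AddLapPoint on the BP_AC_LapManager component of that pawn's controller, if one exists.
; Debug strings print on overlap and registration.
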(event OnComponentBeginOverlap(Box)
  (params (OverlappedComponent :type Primitive%20Component%20Object%20Reference) (OtherActor :type Actor%20Object%20Reference) (OtherComp :type Primitive%20Component%20Object%20Reference) (OtherBodyIndex :type Integer) (bFromSweep :type Boolean) (SweepResult :type Hit%20Result%20Structure%20%28by%20ref%29))
  (Development|PrintString "lappoint")
  (bind _aspawn (Utilities|Casting|CastToPawn OtherActor))
  (Utilities|IsValid (Actor|GetComponentbyClass (Pawn|GetController _aspawn) "/Game/Blueprint/BP_AC_LapManager.BP_AC_LapManager_C")
    (:Is%20Valid
      (Default|AddLapPoint (Actor|GetComponentbyClass (Pawn|GetController _aspawn) "/Game/Blueprint/BP_AC_LapManager.BP_AC_LapManager_C") self)
      (Development|PrintString "Adddlapoitn"))))

(event EventBeginPlay
  (Math|Integer|IncrementInt (Variables|/Game/Blueprint/Player/BP_VehicleAdvGameMode.BP_VehicleAdvGameMode_C|GetLapPointNumber (CallFunction|GetMkGameMode))))

(fn ConstructionScript)