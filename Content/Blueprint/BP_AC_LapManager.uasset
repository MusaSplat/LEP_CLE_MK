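; Actor component that tracks a racer's lap progress in what appears to be a kart race, using lap points crossed along the track.
; AddLapPoint records each unique point; AddLap counts a lap only on the first crossing or when at least 75% of the game mode's lap points were hit, then clears them.
; Each new lap fires OnLapAdded, and exceeding the lap limit calls FinishRace, which only prints a message.
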(event EventBeginPlay)

(event EventTick
  (params (DeltaSeconds :type Float%20%28single-precision%29)))

(fn FinishRace
  (Development|PrintString "Bien joué"))

(fn AddLap
  (Development|PrintString "Bonjour")
  (if (or (>= (Utilities|Array|Length (Variables|Default|GetLapPointCrossed)) (* (Variables|/Game/Blueprint/Player/BP_VehicleAdvGameMode.BP_VehicleAdvGameMode_C|GetLapPointNumber (CallFunction|GetMkGameMode)) 0.75)) (== (Variables|Default|GetCurrentLap) 0))
    (Utilities|Array|Clear (Variables|Default|GetLapPointCrossed))
    (bind _output_get (Variables|Default|SetCurrentLap (+ (Variables|Default|GetCurrentLap) 1)))
    (Default|CallOnLapAdded (Variables|Default|GetCurrentLap))
    (if (> _output_get (Variables|/Game/Blueprint/Player/BP_VehicleAdvGameMode.BP_VehicleAdvGameMode_C|GetNumberOfLap (CallFunction|GetMkGameMode)))
      (CallFunction|FinishRace))))

(fn AddLapPoint
  (params (LapPoint :type BP%20Lap%20Point%20Object%20Reference%20%28by%20ref%29))
  (Utilities|Array|AddUnique (Variables|Default|GetLapPointCrossed) LapPoint))