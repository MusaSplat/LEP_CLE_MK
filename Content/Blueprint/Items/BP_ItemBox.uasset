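; Item box pickup that grants an item to a vehicle pawn driving into it.
; On Cube overlap, it casts the actor to BP_VehicleAdvPawnBase and calls GetItem on the BP_AC_Item_Manager component of that pawn's controller.
; It then hides the cube and disables its collision, restoring visibility and query-only collision after a short delay so the box can be collected again.
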(event OnComponentBeginOverlap(Cube)
  (params (OverlappedComponent :type Primitive%20Component%20Object%20Reference) (OtherActor :type Actor%20Object%20Reference) (OtherComp :type Primitive%20Component%20Object%20Reference) (OtherBodyIndex :type Integer) (bFromSweep :type Boolean) (SweepResult :type Hit%20Result%20Structure%20%28by%20ref%29))
  (bind _asbp_vehicle_adv_pawn_base (Utilities|Casting|CastToBP_VehicleAdvPawnBase OtherActor))
  (Default|GetItem (Actor|GetComponentbyClass (Pawn|GetController _asbp_vehicle_adv_pawn_base) "/Game/Blueprint/Items/BP_AC_Item_Manager.BP_AC_Item_Manager_C"))
  (CallFunction|Disappear))

(event Custom|Disappear
  (bind _cube (Variables|Default|GetCube))
  (bind _cube_2 (Variables|Default|GetCube))
  (Rendering|SetVisibility _cube false false)
  (Collision|SetCollisionEnabled _cube "NoCollision")
  (Utilities|FlowControl|Delay 5.0)
  (Rendering|SetVisibility _cube_2 true false)
  (Collision|SetCollisionEnabled _cube_2 "QueryOnly"))

(fn ConstructionScript)