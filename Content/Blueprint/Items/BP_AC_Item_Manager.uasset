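; Item manager component owned by the vehicle player controller that holds the player's current item.
; GetItem always assigns the banana item, and SetItem stores the item and calls OnItemChange with it.
; UseItem launches the held item with the controller and its controlled vehicle pawn, then clears the slot.
; Tick prints the current item's name on screen as debug output.
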(event EventBeginPlay)

(event EventTick
  (params (DeltaSeconds :type Float%20%28single-precision%29))
  (bind _currentitem (Variables|Default|GetCurrentItem)
    (:then
      (Development|PrintString (Utilities|GetDisplayName _currentitem) true true "(R=1.000000,G=0.203125,B=0.866762,A=1.000000)" 0.0))
    (:else)))

(fn UseItem
  (bind _returnvalue (Components|GetOwner))
  (bind _asbp_vehicle_adv_player_controller (Utilities|Casting|CastToBP_VehicleAdvPlayerController _returnvalue))
  (bind _currentitem (Variables|Default|GetCurrentItem)
    (:then
      (Default|LaunchItem _currentitem _asbp_vehicle_adv_player_controller (.AsBP%20Vehicle%20Adv%20Pawn%20Base (Utilities|Casting|CastToBP_VehicleAdvPawnBase (Pawn|GetControlledPawn _asbp_vehicle_adv_player_controller))))
      (CallFunction|SetItem))
    (:else)))

(fn SetItem
  (params (CurrentItem :type BP%20Item%20Data%20Object%20Reference))
  (bind _output_get (Variables|Default|SetCurrentItem CurrentItem))
  (Default|CallOnItemChange _output_get))

(fn GetItem
  (CallFunction|SetItem "/Game/Data/Items/ID_S_Banana.ID_S_Banana"))